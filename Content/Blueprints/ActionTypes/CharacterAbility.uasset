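; CharacterAbility is an action type for character abilities that spend the user's essence when executed.
; ExecuteAction hands User and Target to UseAbility, which subtracts EssenceCost from the user's CurrentEssence.
; If the user is an AllyUnitBase, it also generates ultimate charge scaled from that cost.
; Target is passed through but not otherwise used here, and no effect on it is applied.
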(event EventBeginPlay
  (|CallParentFunction) ; This node is disabled and will not be called.\nDrag off pins to build functionality.
)

(event EventTick
  (params (DeltaSeconds :type Float%20%28single-precision%29))
  (|CallParentFunction DeltaSeconds) ; This node is disabled and will not be called.\nDrag off pins to build functionality.
)

(fn ExecuteAction
  (params (User :type Unit%20Base%20Object%20Reference) (Target :type Array%20of%20Unit%20Base%20Object%20References))
  (CallFunction|UseAbility User Target) ; Ability consumes essence on use
  (return))

(fn UseAbility
  (params (User :type Unit%20Base%20Object%20Reference) (Target :type Array%20of%20Unit%20Base%20Object%20References))
  (bind _essencecost (Variables|Default|GetEssenceCost))
  (Variables|/Game/Blueprints/UnitBase.UnitBase_C|SetCurrentEssence User (- (Variables|/Game/Blueprints/UnitBase.UnitBase_C|GetCurrentEssence User) _essencecost))
  (bind _asally_unit_base (Utilities|Casting|CastToAllyUnitBase User))
  (Default|GenerateUltCharge _asally_unit_base (/ (Math|Conversions|ToFloat(Integer) _essencecost) 0.75))
  (return))