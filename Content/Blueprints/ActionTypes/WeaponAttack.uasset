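; WeaponAttack is an action type for a unit's weapon attack, used here to build resources on the user.
; ExecuteAction passes User and Target to UseWeaponAttack, which restores a small fixed amount of Essence to the user, then adds ultimate charge if the user is an AllyUnitBase.
; No damage is applied here and Target is unused; the in-graph note's Essence amount differs from the value passed.
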(event EventBeginPlay
  (|CallParentFunction) ; This node is disabled and will not be called.\nDrag off pins to build functionality.
)

(event EventTick
  (params (DeltaSeconds :type Float%20%28single-precision%29))
  (|CallParentFunction DeltaSeconds) ; This node is disabled and will not be called.\nDrag off pins to build functionality.
)

(fn ExecuteAction
  (params (User :type Unit%20Base%20Object%20Reference) (Target :type Array%20of%20Unit%20Base%20Object%20References))
  (CallFunction|UseWeaponAttack User Target) ; Weapon attacks always restore 100 Essence
  (return))

(fn UseWeaponAttack
  (params (User :type Unit%20Base%20Object%20Reference) (Target :type Array%20of%20Unit%20Base%20Object%20References))
  (Default|RegenEssence User 10)
  (bind _asally_unit_base (Utilities|Casting|CastToAllyUnitBase User))
  (Default|GenerateUltCharge _asally_unit_base 2e+01)
  (return))