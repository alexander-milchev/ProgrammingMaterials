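; UnitBase is the base combat unit, holding stats, HP, Essence, shields, statuses and turn-action progress that can be advanced or delayed.
; TakeHit applies damage-taken modifiers, then subtracts Armour or Spiritual Resistance, or multiplies crits while ignoring both.
; TakeDamage drains shields before HP, and crit heals also grant a shield.
; Buffs, debuffs and status effects are added components in one Statuses array, which GetEffectiveStat sums onto base stats.
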(event EventBeginPlay)

(event Collision|EventActorBeginOverlap
  (params (OtherActor :type Actor%20Object%20Reference)))

(event EventTick
  (params (DeltaSeconds :type Float%20%28single-precision%29)))

(fn ConstructionScript
  (Variables|Default|SetTurnActionProgress 0.0)
  (Variables|Default|SetShields (Utilities|Array|MakeArray 0)) ; Sets Shields as empty
  (Variables|Default|SetStatuses (Utilities|Array|MakeArray 0)))

(fn AdvanceAction
  (params (PercentAdvance :type Float%20%28double-precision%29))
  (if (>= (+ PercentAdvance (Variables|Default|GetTurnActionProgress)) 1.0)
    (Variables|Default|SetTurnActionProgress 1.0)
    (else
      (Variables|Default|SetTurnActionProgress (+ PercentAdvance (Variables|Default|GetTurnActionProgress))))))

(fn CalculateDamage
  (params (Damage :type Integer) (Source :type Unit%20Base%20Object%20Reference) (IsCrit :type Boolean) (IsPhysical :type Boolean))
  (if IsPhysical ; Physical or Spiritual Branch
    (if IsCrit ; Crit Armour Ignore
      _
      (else
        ;[1 1 1] Physical DMG calculation
        (bind _post_mitigation_dmg (CallFunction|ArmourMitigation Damage))
        (return _post_mitigation_dmg) ; Return Phys DMG - AR
      ))
    (elif IsCrit ; Crit Resistance Ignore
      _
      (else
        ;[1 1 1] Spiritual DMG calculation
        (bind _post_mitigation_damage (CallFunction|ResistanceMitigation Damage))
        (return _post_mitigation_damage) ; Return Spiritual DMG - SR
      )))
  ;[1 1 1] Critical DMG calculation
  (return (* (Math|Conversions|ToFloat(Integer) Damage) 1.75)) ; Return Crit DMG
)

(fn TakeHit
  (params (Damage :type Integer) (Source :type Unit%20Base%20Object%20Reference) (IsCrit :type Boolean) (Is%20Physical :type Boolean))
  (if IsCrit
    (bind _post_onhit_damage (CallFunction|TakeCritHit Damage Source Is%20Physical)) ; For "On get crit hit" clauses
    (LocalVariables|SetPost%20OnHit%20DMG _post_onhit_damage)
    (elif Is%20Physical
      (bind _post_onhit_dmg (CallFunction|TakePhysHit Source Damage))
      (LocalVariables|SetPost%20OnHit%20DMG _post_onhit_dmg)
      (else
        (bind _post_onhit_dmg_2 (CallFunction|TakeSpiritHit Source Damage))
        (LocalVariables|SetPost%20OnHit%20DMG _post_onhit_dmg_2))))
  (bind _damagereceived (CallFunction|CalculateDamage (LocalVariables|GetPost%20OnHit%20DMG) Source IsCrit Is%20Physical))
  (CallFunction|TakeDamage _damagereceived)
  (return _damagereceived))

(fn TakeCritHit
  (params (Damage :type Integer) (Source :type Unit%20Base%20Object%20Reference) (Is%20Physical :type Boolean))
  (bind _output_get (LocalVariables|SetIntermediate%20DMG Damage))
  (for _array_element (Variables|Default|GetStatuses)
    (bind _asbuff_debuff_base (Utilities|Casting|CastToBuffDebuffBase _array_element))
    ;[1 1 1] General Damage Taken Buff/Debuffs
    (if (Utilities|Enum|Equal(Enum) (Variables|/Game/Blueprints/StatusEffects/BuffDebuffBase.BuffDebuffBase_C|GetTarget%20Stat _asbuff_debuff_base) "NewEnumerator10")
      (if (Variables|/Game/Blueprints/StatusEffects/BuffDebuffBase.BuffDebuffBase_C|GetPositive _asbuff_debuff_base)
        (LocalVariables|SetIntermediate%20DMG (- _output_get (* _output_get (/ (Math|Conversions|ToFloat(Integer) (Variables|/Game/Blueprints/StatusEffects/BuffDebuffBase.BuffDebuffBase_C|GetScaling _asbuff_debuff_base)) 1e+02))))
        (else
          (LocalVariables|SetIntermediate%20DMG (+ _output_get (* _output_get (/ (Math|Conversions|ToFloat(Integer) (Variables|/Game/Blueprints/StatusEffects/BuffDebuffBase.BuffDebuffBase_C|GetScaling _asbuff_debuff_base)) 1e+02))))))
      (elif (Utilities|Enum|Equal(Enum) (Variables|/Game/Blueprints/StatusEffects/BuffDebuffBase.BuffDebuffBase_C|GetTarget%20Stat _asbuff_debuff_base) "NewEnumerator8")
        ;[1 1 1] Physical Damage Taken
        (if Is%20Physical ; Only if DMG is also physical
          (if (Variables|/Game/Blueprints/StatusEffects/BuffDebuffBase.BuffDebuffBase_C|GetPositive _asbuff_debuff_base)
            (LocalVariables|SetIntermediate%20DMG (- _output_get (* _output_get (/ (Math|Conversions|ToFloat(Integer) (Variables|/Game/Blueprints/StatusEffects/BuffDebuffBase.BuffDebuffBase_C|GetScaling _asbuff_debuff_base)) 1e+02))))
            (else
              (LocalVariables|SetIntermediate%20DMG (+ _output_get (* _output_get (/ (Math|Conversions|ToFloat(Integer) (Variables|/Game/Blueprints/StatusEffects/BuffDebuffBase.BuffDebuffBase_C|GetScaling _asbuff_debuff_base)) 1e+02)))))))
        (elif (Utilities|Enum|Equal(Enum) (Variables|/Game/Blueprints/StatusEffects/BuffDebuffBase.BuffDebuffBase_C|GetTarget%20Stat _asbuff_debuff_base) "NewEnumerator9")
          ;[1 1 1] Spiritual Damage Taken
          (if (not Is%20Physical) ; Only if DMG is also Spiritual
            (if (Variables|/Game/Blueprints/StatusEffects/BuffDebuffBase.BuffDebuffBase_C|GetPositive _asbuff_debuff_base)
              (LocalVariables|SetIntermediate%20DMG (- _output_get (* _output_get (/ (Math|Conversions|ToFloat(Integer) (Variables|/Game/Blueprints/StatusEffects/BuffDebuffBase.BuffDebuffBase_C|GetScaling _asbuff_debuff_base)) 1e+02))))
              (else
                (LocalVariables|SetIntermediate%20DMG (+ _output_get (* _output_get (/ (Math|Conversions|ToFloat(Integer) (Variables|/Game/Blueprints/StatusEffects/BuffDebuffBase.BuffDebuffBase_C|GetScaling _asbuff_debuff_base)) 1e+02)))))))))))
  (return (LocalVariables|GetIntermediate%20DMG)))

(fn ReceiveHealing
  (params (Heal :type Integer) (Source :type Unit%20Base%20Object%20Reference) (Is%20Crit :type Boolean))
  (if Is%20Crit
    (CallFunction|ReceiveShield (Math|Float|Truncate (* (Math|Conversions|ToFloat(Integer) Heal) 0.75)) Source 99))
  (bind _stat (CallFunction|GetEffectiveStat "NewEnumerator0"))
  (if (> (+ (Variables|Default|GetCurrentHP) Heal) _stat)
    (Variables|Default|SetCurrentHP _stat)
    (else
      (Variables|Default|SetCurrentHP (+ (Variables|Default|GetCurrentHP) Heal)))))

(fn ReceiveShield
  (params (Shield :type Integer) (Source :type Unit%20Base%20Object%20Reference) (Duration :type Integer))
  (bind _returnvalue (AddComponent|AddShield))
  (LocalVariables|SetNew%20Shield _returnvalue)
  (Variables|/Game/Blueprints/StatusEffects/Shield.Shield_C|SetShield%20HP (LocalVariables|GetNew%20Shield) Shield)
  (Variables|/Game/Blueprints/StatusEffects/Shield.Shield_C|SetSource (LocalVariables|GetNew%20Shield) Source)
  (Variables|/Game/Blueprints/StatusEffects/Shield.Shield_C|SetDuration (LocalVariables|GetNew%20Shield) Duration)
  (Utilities|Array|Add (Variables|Default|GetShields) (LocalVariables|GetNew%20Shield))
  (return))

(fn TakeDamage
  (params (Damage :type Integer))
  (bind _shields (Variables|Default|GetShields))
  (LocalVariables|SetIntermediateDMG Damage)
  (if (Utilities|Array|IsEmpty _shields) ; If no shields, skip to damaging HP
    ;[1 1 1] Current HP - Intermediate DMG
    (Variables|Default|SetCurrentHP (- (Variables|Default|GetCurrentHP) (LocalVariables|GetIntermediateDMG)) :!label _label)
    (return)
    (else
      (bind (_array_element _array_index) (Utilities|Array|ForEachLoopwithBreak _shields :!label _label_2)
        (:LoopBody
          (if (<= (Variables|/Game/Blueprints/StatusEffects/Shield.Shield_C|GetShield%20HP _array_element) (LocalVariables|GetIntermediateDMG))
            ;[1 1 1] Shield Destroyed (DMG >= Shield)
            (LocalVariables|SetIntermediateDMG (- (LocalVariables|GetIntermediateDMG) (Variables|/Game/Blueprints/StatusEffects/Shield.Shield_C|GetShield%20HP _array_element)))
            (Utilities|Array|RemoveIndex _shields _array_index) ; Destroy current shield and reduce intermediate dmg
            (else
              ;[1 1 1] Shield(s) survive damage (DMG < Shield)
              (Variables|/Game/Blueprints/StatusEffects/Shield.Shield_C|SetShield%20HP _array_element (- (Variables|/Game/Blueprints/StatusEffects/Shield.Shield_C|GetShield%20HP _array_element) (LocalVariables|GetIntermediateDMG))) ; Shield survives DMG, no more damage to calculate
              (LocalVariables|SetIntermediateDMG 0)
              (goto _label_2 Break))))
        (:Completed
          (goto _label))))))

(fn DelayAction
  (params (Delay%20Amount :type Float%20%28double-precision%29))
  (Variables|Default|SetTurnActionProgress (- (Variables|Default|GetTurnActionProgress) Delay%20Amount)))

(fn ArmourMitigation
  (params (Damage :type Integer))
  (bind _stat (CallFunction|GetEffectiveStat "NewEnumerator5"))
  (return (- Damage _stat)))

(fn ResistanceMitigation
  (params (Damage :type Integer))
  (bind _stat (CallFunction|GetEffectiveStat "NewEnumerator6"))
  (return (- Damage _stat)))

(fn CalcMaxHP
  (params (BaseMaxHP :type Integer))
  (bind _output_get (Variables|Default|SetMaxHealth BaseMaxHP))
  (Variables|Default|SetCurrentHP _output_get))

(fn CalcMaxEssence
  (params (BaseMaxEssence :type Integer))
  (bind _output_get (Variables|Default|SetMaxEssence BaseMaxEssence))
  (Variables|Default|SetCurrentEssence _output_get))

(fn TakePhysHit
  (params (Source :type Unit%20Base%20Object%20Reference) (Damage :type Integer))
  (bind _output_get (LocalVariables|SetIntermediate%20DMG Damage))
  (for _array_element (Variables|Default|GetStatuses)
    (bind _asbuff_debuff_base (Utilities|Casting|CastToBuffDebuffBase _array_element))
    (if (Utilities|Enum|Equal(Enum) (Variables|/Game/Blueprints/StatusEffects/BuffDebuffBase.BuffDebuffBase_C|GetTarget%20Stat _asbuff_debuff_base) "NewEnumerator10")
      (if (Variables|/Game/Blueprints/StatusEffects/BuffDebuffBase.BuffDebuffBase_C|GetPositive _asbuff_debuff_base)
        (LocalVariables|SetIntermediate%20DMG (- (LocalVariables|GetIntermediate%20DMG) (* _output_get (/ (Math|Conversions|ToFloat(Integer) (Variables|/Game/Blueprints/StatusEffects/BuffDebuffBase.BuffDebuffBase_C|GetScaling _asbuff_debuff_base)) 1e+02))))
        (else
          (LocalVariables|SetIntermediate%20DMG (+ (LocalVariables|GetIntermediate%20DMG) (* _output_get (/ (Math|Conversions|ToFloat(Integer) (Variables|/Game/Blueprints/StatusEffects/BuffDebuffBase.BuffDebuffBase_C|GetScaling _asbuff_debuff_base)) 1e+02))))))
      (elif (Utilities|Enum|Equal(Enum) (Variables|/Game/Blueprints/StatusEffects/BuffDebuffBase.BuffDebuffBase_C|GetTarget%20Stat _asbuff_debuff_base) "NewEnumerator9")
        (if (Variables|/Game/Blueprints/StatusEffects/BuffDebuffBase.BuffDebuffBase_C|GetPositive _asbuff_debuff_base)
          (LocalVariables|SetIntermediate%20DMG (- (LocalVariables|GetIntermediate%20DMG) (* _output_get (/ (Math|Conversions|ToFloat(Integer) (Variables|/Game/Blueprints/StatusEffects/BuffDebuffBase.BuffDebuffBase_C|GetScaling _asbuff_debuff_base)) 1e+02))))
          (else
            (LocalVariables|SetIntermediate%20DMG (+ (LocalVariables|GetIntermediate%20DMG) (* _output_get (/ (Math|Conversions|ToFloat(Integer) (Variables|/Game/Blueprints/StatusEffects/BuffDebuffBase.BuffDebuffBase_C|GetScaling _asbuff_debuff_base)) 1e+02)))))))))
  (return _output_get))

(fn TakeSpiritHit
  (params (Source :type Unit%20Base%20Object%20Reference) (Damage :type Integer))
  (bind _output_get (Variables|Default|SetIntermediate%20DMG Damage))
  (for _array_element (Variables|Default|GetStatuses)
    (bind _asbuff_debuff_base (Utilities|Casting|CastToBuffDebuffBase _array_element))
    (if (Utilities|Enum|Equal(Enum) (Variables|/Game/Blueprints/StatusEffects/BuffDebuffBase.BuffDebuffBase_C|GetTarget%20Stat _asbuff_debuff_base) "NewEnumerator10")
      (if (Variables|/Game/Blueprints/StatusEffects/BuffDebuffBase.BuffDebuffBase_C|GetPositive _asbuff_debuff_base)
        (Variables|Default|SetIntermediate%20DMG (- (Variables|Default|GetIntermediate%20DMG) (* _output_get (/ (Math|Conversions|ToFloat(Integer) (Variables|/Game/Blueprints/StatusEffects/BuffDebuffBase.BuffDebuffBase_C|GetScaling _asbuff_debuff_base)) 1e+02))))
        (else
          (Variables|Default|SetIntermediate%20DMG (+ (Variables|Default|GetIntermediate%20DMG) (* _output_get (/ (Math|Conversions|ToFloat(Integer) (Variables|/Game/Blueprints/StatusEffects/BuffDebuffBase.BuffDebuffBase_C|GetScaling _asbuff_debuff_base)) 1e+02))))))
      (elif (Utilities|Enum|Equal(Enum) (Variables|/Game/Blueprints/StatusEffects/BuffDebuffBase.BuffDebuffBase_C|GetTarget%20Stat _asbuff_debuff_base) "NewEnumerator9")
        (if (Variables|/Game/Blueprints/StatusEffects/BuffDebuffBase.BuffDebuffBase_C|GetPositive _asbuff_debuff_base)
          (Variables|Default|SetIntermediate%20DMG (- (Variables|Default|GetIntermediate%20DMG) (* _output_get (/ (Math|Conversions|ToFloat(Integer) (Variables|/Game/Blueprints/StatusEffects/BuffDebuffBase.BuffDebuffBase_C|GetScaling _asbuff_debuff_base)) 1e+02))))
          (else
            (Variables|Default|SetIntermediate%20DMG (+ (Variables|Default|GetIntermediate%20DMG) (* _output_get (/ (Math|Conversions|ToFloat(Integer) (Variables|/Game/Blueprints/StatusEffects/BuffDebuffBase.BuffDebuffBase_C|GetScaling _asbuff_debuff_base)) 1e+02)))))))))
  (return _output_get))

(fn RegenEssence
  (params (Regen%20Ammount :type Integer))
  (bind _stat (CallFunction|GetEffectiveStat "NewEnumerator1"))
  (if (< _stat (+ Regen%20Ammount (Variables|Default|GetCurrentEssence)))
    (Variables|Default|SetCurrentEssence _stat)
    (else
      (Variables|Default|SetCurrentEssence (+ Regen%20Ammount (Variables|Default|GetCurrentEssence)))))
  (return))

(fn GetEffectiveStat
  (params (Target%20Stat :type StatTarget%20Enum :default "NewEnumerator0"))
  (LocalVariables|SetStat%20Keeper 0)
  (for _array_element (Variables|Default|GetStatuses)
    (bind _asbuff_debuff_base (Utilities|Casting|CastToBuffDebuffBase _array_element))
    (if (Utilities|Enum|Equal(Enum) (Variables|/Game/Blueprints/StatusEffects/BuffDebuffBase.BuffDebuffBase_C|GetTarget%20Stat _asbuff_debuff_base) Target%20Stat)
      (if (Variables|/Game/Blueprints/StatusEffects/BuffDebuffBase.BuffDebuffBase_C|GetPositive _asbuff_debuff_base)
        (LocalVariables|SetStat%20Keeper (+ (LocalVariables|GetStat%20Keeper) (Variables|/Game/Blueprints/StatusEffects/BuffDebuffBase.BuffDebuffBase_C|GetScaling _asbuff_debuff_base)))
        (else
          (LocalVariables|SetStat%20Keeper (- (LocalVariables|GetStat%20Keeper) (Variables|/Game/Blueprints/StatusEffects/BuffDebuffBase.BuffDebuffBase_C|GetScaling _asbuff_debuff_base)))))))
  (switch Utilities|FlowControl|Switch|SwitchonStatTarget Target%20Stat
    (:NewEnumerator0
      (return (+ (Variables|Default|GetMaxHealth) (LocalVariables|GetStat%20Keeper))))
    (:NewEnumerator1
      (return (+ (Variables|Default|GetMaxEssence) (LocalVariables|GetStat%20Keeper))))
    (:NewEnumerator2
      (return (+ (Variables|Default|GetStrength) (LocalVariables|GetStat%20Keeper))))
    (:NewEnumerator3
      (return (+ (Variables|Default|GetSpiritualAptitude) (LocalVariables|GetStat%20Keeper))))
    (:NewEnumerator4
      (return (+ (Variables|Default|GetSpeed) (LocalVariables|GetStat%20Keeper))))
    (:NewEnumerator5
      (return (+ (Variables|Default|GetArmour) (LocalVariables|GetStat%20Keeper))))
    (:NewEnumerator6
      (return (+ (Variables|Default|GetSpiritualResistance) (LocalVariables|GetStat%20Keeper))))
    (:NewEnumerator7
      (return (+ (Variables|Default|GetCritChance) (LocalVariables|GetStat%20Keeper))))))

(fn ApplyStatusEffect
  (params (Caster :type Unit%20Base%20Object%20Reference) (Duration :type Integer) (Status%20Type :type StatusEffectType%20Enum :default "NewEnumerator0") (Disspellable :type Boolean))
  (bind _returnvalue (AddComponent|AddNonScalingStatusBase))
  (Default|CreateStatus _returnvalue Caster Duration Disspellable)
  (Variables|/Game/Blueprints/StatusEffects/NonScalingStatusBase.NonScalingStatusBase_C|SetStatus%20Effect _returnvalue Status%20Type)
  (Utilities|Array|Add (Variables|Default|GetStatuses) _returnvalue)
  (return))

(fn ApplyBuffDebuff
  (params (Source :type Unit%20Base%20Object%20Reference) (Positive :type Boolean) (Target%20Stat :type StatTarget%20Enum :default "NewEnumerator0") (Scale :type Integer) (Duration :type Integer) (Disspellable :type Boolean))
  (bind _returnvalue (AddComponent|AddBuffDebuffBase))
  (Default|CreateStatus _returnvalue Source Duration Disspellable)
  (Variables|/Game/Blueprints/StatusEffects/BuffDebuffBase.BuffDebuffBase_C|SetPositive _returnvalue Positive)
  (Variables|/Game/Blueprints/StatusEffects/BuffDebuffBase.BuffDebuffBase_C|SetTarget%20Stat _returnvalue Target%20Stat)
  (Variables|/Game/Blueprints/StatusEffects/BuffDebuffBase.BuffDebuffBase_C|SetScaling _returnvalue Scale)
  (Utilities|Array|Add (Variables|Default|GetStatuses) _returnvalue)
  (return))