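; Turn queue Blueprint for a turn-based battle, deciding which unit acts next.
; TurnRequest appends units to TurnOrder, and StartTurn uses a DoOnce gate to call StartUnitTurn on the first unit's CombatComponent.
; ReadyNextTurn resets the gate and starts a turn if the queue has an entry.
; Nodes for binding turn-ended and removing the first entry are unconnected, so this graph never dequeues units.
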(event Custom|TurnRequest
  (params (Unit :type Unit%20Base%20Object%20Reference))
  (Utilities|Array|Add (Variables|Default|GetTurnOrder) Unit)
  (CallFunction|StartTurn))

(event Custom|StartTurn
  (Utilities|FlowControl|DoOnce false
    (:Completed
      (if (Utilities|Array|IsValidIndex (Variables|Default|GetTurnOrder))
        (Default|StartUnitTurn (Variables|/Game/Blueprints/UnitBase.UnitBase_C|GetCombatComponent (Utilities|Array|Get(acopy) (Variables|Default|GetTurnOrder))))))))

(event Custom|ReadyNextTurn
  (Utilities|FlowControl|Sequence
    (:then_0
      (Utilities|FlowControl|DoOnce false) ; enters at Reset
    )
    (:then_1
      (if (Utilities|Array|IsValidIndex (Variables|Default|GetTurnOrder))
        (CallFunction|StartTurn)))))

(event EventBeginPlay)

(event EventTick
  (params (DeltaSeconds :type Float%20%28single-precision%29)))

(fn ConstructionScript)