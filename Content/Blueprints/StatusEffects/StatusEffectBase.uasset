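; StatusEffectBase is an actor component Blueprint that provides the base logic for a timed status effect.
; CreateStatus stores the caster as Source, along with the duration and whether the effect is disspellable.
; Each TickDown call lowers Duration by one, calls RemoveStatus to destroy the component on expiry, and returns whether it expired.
; BeginPlay and Tick are unused, so the countdown depends on outside calls to TickDown.
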(event EventBeginPlay)

(event EventTick
  (params (DeltaSeconds :type Float%20%28single-precision%29)))

(fn CreateStatus
  (params (Caster :type Unit%20Base%20Object%20Reference) (Duration :type Integer) (Disspellable :type Boolean))
  (Variables|Default|SetSource Caster)
  (Variables|Default|SetDuration Duration)
  (Variables|Default|SetDisspellable Disspellable)
  (return))

(fn RemoveStatus
  (Components|DestroyComponent)
  (return))

(fn TickDown
  (bind _output_get (Variables|Default|SetDuration (- (Variables|Default|GetDuration) 1)))
  (if (<= _output_get 0)
    (CallFunction|RemoveStatus))
  (return (<= _output_get 0)))